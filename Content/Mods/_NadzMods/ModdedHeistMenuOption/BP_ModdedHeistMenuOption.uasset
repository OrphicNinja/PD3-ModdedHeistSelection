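; Mod actor that adds a "Modded Heists" button to the CrimeNet main menu, opening a selection screen for mod-installed heists.
; BeginPlay collects heists with level paths under /Game/Mods, flags them as tutorial levels and builds their list buttons.
; Tick scans for CrimeNet menu widgets and injects the button when missing.
; Hover updates description and banner, with a placeholder fallback; selection requests a solo game at the chosen difficulty.
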(event `self.ReceiveBeginPlay`
  (bind _returnvalue (`|CreateWidget` "/Game/UI/Widgets/Menus/Buttons/WBP_UI_CrimeNet_TextButton.WBP_UI_CrimeNet_TextButton_C"))
  (set `self.ModdedHeistButton` _returnvalue)
  (bind _returnvalue_2 (`|CreateWidget` "/Game/Mods/_NadzMods/ModdedHeistMenuOption/UI/WBP_UI_ModdedHeists_HeistSelection.WBP_UI_ModdedHeists_HeistSelection_C"))
  (set `self.ModdedHeistsMenu` _returnvalue_2)
  (`self.GetHeistInfo`)
  (`self.MakeModdedHeistButtons`)
  (for _array_element (`self.HeistDataButtonsArray`)
    (`PanelWidget.AddChild` (`/Game/Mods/_NadzMods/ModdedHeistMenuOption/UI/WBP_UI_ModdedHeists_HeistSelection.ScrollBox_LevelList` (`self.ModdedHeistsMenu`)) _array_element)
    (bind _output_get (set `self.SelectedButton` (`|GetArrayItem` (`self.HeistDataButtonsArray`))))
    (`self.SetSelectedHeistInfo` _output_get)))

(event `self.ReceiveTick`
  (params (DeltaSeconds :type "Float (single-precision)"))
  (`self.AddHeistButtonToMenu`))

(event `OnMainMenuButtonSelected`
  (params (Button :type "SBZMenuButton Object Reference"))
  (`UserWidget.AddToViewport` (`self.ModdedHeistsMenu`) 0))

(event `OnButtonHover`
  (params (Button :type "SBZMenuButton Object Reference") (bIsEnabled :type Boolean))
  (bind _aswbp_ui_heist_button (cast `/Game/Mods/_NadzMods/ModdedHeistMenuOption/UI/WBP_UI_HeistButton` Button))
  (bind _output_get (set `self.SelectedButton` _aswbp_ui_heist_button))
  (`self.SetSelectedHeistInfo` _output_get))

(event `OnHeistButtonSelected`
  (params (Button :type "SBZMenuButton Object Reference"))
  (`Widget.SetVisibility` (`/Game/Mods/_NadzMods/ModdedHeistMenuOption/UI/WBP_UI_ModdedHeists_HeistSelection.Overlay_PanelSpace` (`self.ModdedHeistsMenu`)) "Collapsed")
  (`Widget.SetVisibility` (`/Game/Mods/_NadzMods/ModdedHeistMenuOption/UI/WBP_UI_ModdedHeists_HeistSelection.Overlay_HeistDescription` (`self.ModdedHeistsMenu`)) "Collapsed")
  (bind _aswbp_ui_heist_button (cast `/Game/Mods/_NadzMods/ModdedHeistMenuOption/UI/WBP_UI_HeistButton` Button))
  (bind _returnvalue (`SBZGameUserSettings.Get`))
  (`SBZGameStateMachine.RequestSoloGame` (`SBZGameInstance.GameStateMachine` (`SBZGameUserSettings.GameInstance` _returnvalue)) (`SBZGameStateMachineSettings.LevelPathToIdx` (`PD3HeistDataAsset.LevelPath` (`/Game/Mods/_NadzMods/ModdedHeistMenuOption/UI/WBP_UI_HeistButton.HeistDataAsset` _aswbp_ui_heist_button))) (`/Game/Mods/_NadzMods/ModdedHeistMenuOption/UI/WBP_UI_ModdedHeists_HeistSelection.CurrentDifficultyIndex` (`self.ModdedHeistsMenu`))))

(fn `AddHeistButtonToMenu`
  (bind _moddedheistbutton (`self.ModdedHeistButton`))
  (bind _foundwidgets (`WidgetBlueprintLibrary.GetAllWidgetsOfClass` "/Game/UI/Widgets/StateMachine/GameStart/WBP_UI_MainMenu_CrimeNet.WBP_UI_MainMenu_CrimeNet_C" false))
  (for _array_element _foundwidgets
    (bind _asvertical_box (cast `VerticalBox` (`PanelWidget.GetChildAt` (`/Game/UI/Widgets/StateMachine/GameStart/WBP_UI_MainMenu_CrimeNet.Overlay_SelectHeist` _array_element) 0)))
    (if (not (`PanelWidget.HasChild` _asvertical_box (`self.ModdedHeistButton`)))
      (`/Game/UI/Widgets/Menus/Buttons/WBP_UI_CrimeNet_TextButton.SetButtonText` _moddedheistbutton "Modded Heists")
      (`/Game/UI/Widgets/Menus/Buttons/WBP_UI_CrimeNet_TextButton.SetTextDescription` _moddedheistbutton "Play one of the heists you modded in")
      (set `/Game/UI/Widgets/Menus/Buttons/WBP_UI_CrimeNet_TextButton.PaperSprite_Image_Buttons` "/Game/Mods/_NadzMods/ModdedHeistMenuOption/UI/Textures/SS_UI_ModdedHeists_Button.SS_UI_ModdedHeists_Button" _moddedheistbutton)
      (add `SBZMenuButton.OnButtonSelected` _moddedheistbutton (`|CreateDelegate` :!event `OnMainMenuButtonSelected`))
      (`PanelWidget.AddChild` _asvertical_box _moddedheistbutton))))

(fn `GetHeistInfo`
  (for _array_element (`SBZHeistDeveloperSettings.GetAllHeistData`)
    (bind (_heistdata _levelpath) (break `SBZHeistDataLevelPair` _array_element))
    (if (`KismetStringLibrary.Contains` (`KismetSystemLibrary.BreakSoftObjectPath` _levelpath) "/Game/Mods")
      (set `PD3HeistDataAsset.bIsTutorialLevel` true _heistdata)
      (`KismetArrayLibrary.Array_Add` (`self.ModdedHeistsArray`) _array_element))))

(fn `MakeModdedHeistButtons`
  (for _array_element (`self.ModdedHeistsArray`)
    (bind _returnvalue (`|CreateWidget` "/Game/Mods/_NadzMods/ModdedHeistMenuOption/UI/WBP_UI_HeistButton.WBP_UI_HeistButton_C" null 24 "/Game/UI/Assets/Fonts/Din_Pro/DINPro-CondMedium_Font.DINPro-CondMedium_Font" null))
    (bind _heistdata (break `SBZHeistDataLevelPair` _array_element))
    (set `/Game/Mods/_NadzMods/ModdedHeistMenuOption/UI/WBP_UI_HeistButton.HeistDataAsset` _heistdata _returnvalue)
    (bind _heistdisplayname (`PD3HeistDataAsset.HeistDisplayName` _heistdata))
    (`TextBlock.SetText` (`/Game/Mods/_NadzMods/ModdedHeistMenuOption/UI/WBP_UI_HeistButton.Text_DisplayText` _returnvalue) _heistdisplayname)
    (`/Game/Mods/_NadzMods/ModdedHeistMenuOption/UI/WBP_UI_HeistButton.SetButtonText` _returnvalue _heistdisplayname)
    (add `SBZMenuButton.OnButtonSelected` _returnvalue (`|CreateDelegate` :!event `OnHeistButtonSelected`))
    (add `SBZMenuButton.OnButtonFocusedChanged` _returnvalue (`|CreateDelegate` :!event `OnButtonHover`))
    (`KismetArrayLibrary.Array_Add` (`self.HeistDataButtonsArray`) _returnvalue)))

(fn `SetSelectedHeistInfo`
  (params (SelectedButton :type "/Game/Mods/_NadzMods/ModdedHeistMenuOption/UI/WBP_UI_HeistButton Object Reference"))
  (bind _moddedheistsmenu (`self.ModdedHeistsMenu`))
  (bind _heistdataasset (`/Game/Mods/_NadzMods/ModdedHeistMenuOption/UI/WBP_UI_HeistButton.HeistDataAsset` SelectedButton))
  (bind _image_levelicon (`/Game/Mods/_NadzMods/ModdedHeistMenuOption/UI/WBP_UI_ModdedHeists_HeistSelection.Image_LevelIcon` _moddedheistsmenu))
  (bind _output (`|ConvertAsset` (`PD3HeistDataAsset.HeistBannerImage` _heistdataasset)))
  (`TextBlock.SetText` (`/Game/Mods/_NadzMods/ModdedHeistMenuOption/UI/WBP_UI_ModdedHeists_HeistSelection.Text_Desc_LevelDescription` _moddedheistsmenu) (`PD3HeistDataAsset.HeistDescription` _heistdataasset))
  (if (== _output null)
    (`Image.SetBrush` _image_levelicon (`PaperSpriteBlueprintLibrary.MakeBrushFromSprite` "/Game/Mods/_NadzMods/ModdedHeistMenuOption/UI/Textures/SS_UI_Placeholder_Banner_Sprite.SS_UI_Placeholder_Banner_Sprite" 512 256))
    (else
      (`Image.SetBrush` _image_levelicon (`PaperSpriteBlueprintLibrary.MakeBrushFromSprite` _output 512 256)))))

(fn `UserConstructionScript`)